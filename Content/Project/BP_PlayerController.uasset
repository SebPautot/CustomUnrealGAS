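; Player controller Blueprint that builds the gameplay HUD and fills it with buttons for the possessed pawn's abilities.
; On possess, it binds to the pawn AbilitySystem's all-abilities-initialized event, then creates WBP_Gameplay and adds it to the player screen.
; When that event fires, it creates a WBP_AbilityButton for each ability, hands it the ability and HUD references, and adds it to the HUD.
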(event `self.ReceivePossess`
  (params (PossessedPawn :type "Pawn Object Reference"))
  (add `ASAbilitySystem.OnAllAbilitiesInitialized` (`ASPawn.AbilitySystem` (`self.GetPlayerPawn`)) (delegate `Abilities Ready`))
  (bind _returnvalue (`|CreateWidget` "/Game/Project/UI/WBP_Gameplay.WBP_Gameplay_C" self))
  (bind _output_get (set `self.Hud` _returnvalue))
  (`UserWidget.AddToPlayerScreen` _output_get 0))

(event `Abilities Ready`
  (bind _hud (`self.Hud`))
  (bind _values (`BlueprintMapLibrary.Map_Values` (`ASAbilitySystem.Abilities` (`ASPawn.AbilitySystem` (`self.GetPlayerPawn`)))))
  (for _array_element _values
    (bind _returnvalue (`|CreateWidget` "/Game/Project/UI/WBP_AbilityButton.WBP_AbilityButton_C" self _array_element))
    (`/Game/Project/UI/WBP_AbilityButton.SetAbilityButtonData` _returnvalue _array_element _hud)
    (`/Game/Project/UI/WBP_Gameplay.Add child ability` _hud _returnvalue)))

(fn `UserConstructionScript`)