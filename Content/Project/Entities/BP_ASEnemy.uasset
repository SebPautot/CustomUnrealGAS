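; BP_ASEnemy is an enemy Blueprint that shows its health through a WBP_EnemyHealth widget.
; On BeginPlay it binds to the HealthComponent's health-changed event and caches the widget from its Widget component.
; Health changes push the new value and max health to the widget, and OnLevelSet refreshes it from the component's current values.
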(event `self.ReceiveBeginPlay`
  (add `ASHealthComponent.OnHealthChanged` (`self.HealthComponent`) (delegate `OnHealthChanged_Event`))
  (bind _aswbp_enemy_health (cast `/Game/Project/UI/WBP_EnemyHealth` (`WidgetComponent.GetWidget` (`self.Widget`))))
  (set `self.EnemyHealth` _aswbp_enemy_health))

(event `OnHealthChanged_Event`
  (params (HealthComponent :type "ASHealthComponent Object Reference") (Health :type "Float (single-precision)"))
  (`/Game/Project/UI/WBP_EnemyHealth.SetHealth` (`self.EnemyHealth`) Health (`ASHealthComponent.MaxHealth` HealthComponent)))

(event `self.OnLevelSet`
  (bind _healthcomponent (`self.HealthComponent`))
  (`/Game/Project/UI/WBP_EnemyHealth.SetHealth` (`self.EnemyHealth`) (`ASHealthComponent.Health` _healthcomponent) (`ASHealthComponent.MaxHealth` _healthcomponent)))

(fn `UserConstructionScript`)